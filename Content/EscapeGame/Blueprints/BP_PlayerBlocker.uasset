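; BP_PlayerBlocker is an actor whose static mesh slides along a movement offset while something overlaps its box, and slides back when the overlap ends.
; Box overlap events set the overlap flag and flip the sign of the angular speed, without filtering which actor overlaps.
; Tick advances an angle clamped to a quarter turn and uses its sine to ease the mesh between its initial and displaced locations.
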(event OnComponentBeginOverlap(Box)
  (params (OverlappedComponent :type Primitive%20Component%20Object%20Reference) (OtherActor :type Actor%20Object%20Reference) (OtherComp :type Primitive%20Component%20Object%20Reference) (OtherBodyIndex :type Integer) (bFromSweep :type Boolean) (SweepResult :type Hit%20Result%20Structure%20%28by%20ref%29))
  (bind _angleperseconds (Variables|Default|GetAnglePerSeconds))
  (Variables|Default|SetOverlapping true)
  (if (< _angleperseconds 0.0)
    (Math|Float|NegateFloat _angleperseconds)))

(event OnComponentEndOverlap(Box)
  (params (OverlappedComponent :type Primitive%20Component%20Object%20Reference) (OtherActor :type Actor%20Object%20Reference) (OtherComp :type Primitive%20Component%20Object%20Reference) (OtherBodyIndex :type Integer))
  (Variables|Default|SetOverlapping false)
  (Math|Float|NegateFloat (Variables|Default|GetAnglePerSeconds)))

(event EventBeginPlay
  (Variables|Default|SetInitialOffset (Variables|/Script/Engine.SceneComponent|GetRelativeLocation (Variables|Default|GetStaticMesh))))

(event EventTick
  (params (DeltaSeconds :type Float%20%28single-precision%29))
  (if (Math|Boolean|ANDBoolean (>= (Variables|Default|GetAngle) 0.0) (< (Variables|Default|GetAngle) 9e+01) (Variables|Default|GetOverlapping))
    (bind _output_get (Variables|Default|SetAngle (Math|Float|Clamp(Float) (+ (Variables|Default|GetAngle) (* DeltaSeconds (Variables|Default|GetAnglePerSeconds))) 0.0 9e+01) :!label _label))
    (Transformation|SetRelativeLocation (Variables|Default|GetStaticMesh) (+ (* (Variables|Default|GetMovementAmount) (Math|Trig|Sin(Degrees) _output_get)) (Variables|Default|GetInitialOffset)) false false)
    (elif (Math|Boolean|ANDBoolean (< (Variables|Default|GetAnglePerSeconds) 0.0) (> (Variables|Default|GetAngle) 0.0) (not (Variables|Default|GetOverlapping)))
      (goto _label))))

(fn ConstructionScript)
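; BP_Door is an escape game door that slides its SMDoorCasing mesh vertically between open and closed positions.
; BeginPlay caches the start location and derives a raised end location.
; Each Trigger event flips the Opened/Closed state and plays or reverses a timeline that lerps the casing between those locations.
; An unconnected item-pickup gameplay message listener only prints a test string and never runs.
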(event EventTrigger
  (switch Utilities|FlowControl|Switch|SwitchonOpenClosed_Enum (Variables|Default|GetState)
    (:NewEnumerator0
      (Variables|Default|SetState (Utilities|Select :Index (Variables|Default|GetState) :NewEnumerator0 "NewEnumerator1" :NewEnumerator1 "NewEnumerator0"))
      (bind _alpha (Timeline|OpenCloseTimeline Reverse)
        (:Update
          (Transformation|SetRelativeLocation (Variables|Default|GetSM_DoorCasing) (Math|Vector|Lerp(Vector) (Variables|Default|GetInitialLocation) (Variables|Default|GetEndLocation) _alpha) false false))))
    (:NewEnumerator1
      (Variables|Default|SetState (Utilities|Select :Index (Variables|Default|GetState) :NewEnumerator0 "NewEnumerator1" :NewEnumerator1 "NewEnumerator0"))
      (Timeline|OpenCloseTimeline Play))))

(event EventBeginPlay
  (bind _output_get (Variables|Default|SetInitialLocation (Variables|/Script/Engine.SceneComponent|GetRelativeLocation (Variables|Default|GetSM_DoorCasing))))
  (Variables|Default|SetEndLocation (+ _output_get "0,0,301.000000")))

(fn ConstructionScript)
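; BP_Furniture_Base is the base furniture Blueprint in EscapeGame, providing interaction prompts for drawers and cabinet doors.
; A component counts as interactive if it resolves to an entry in Drawers or CabinetDoors.
; GetInteractionText picks open or close wording from that entry's state, or returns an error string when nothing matches.
; Focus events show that text on the player character's HUD and hide the widget when focus ends.
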(event EventOnBeginFocus
  (params (Controller :type Controller%20Object%20Reference) (Comp :type Actor%20Component%20Object%20Reference))
  (bind _returnvalue (CallFunction|GetInteractionText Comp))
  (if (Utilities|Enum|NotEqual(Enum) _returnvalue (Variables|Default|GetInteractionTextErrString))
    (bind _asbp_player_character (Utilities|Casting|CastToBP_PlayerCharacter (Pawn|GetControlledPawn Controller)))
    (Default|ToggleInteractWidget (Variables|/Game/EscapeGame/Blueprints/BP_PlayerCharacter.BP_PlayerCharacter_C|GetHUD _asbp_player_character) "Visible")
    (Default|SetInteractText (Variables|/Game/EscapeGame/Blueprints/BP_PlayerCharacter.BP_PlayerCharacter_C|GetHUD _asbp_player_character) _returnvalue)))

(event EventOnEndFocus
  (params (Controller :type Controller%20Object%20Reference))
  (bind _asbp_player_character (Utilities|Casting|CastToBP_PlayerCharacter (Pawn|GetControlledPawn Controller)))
  (Default|ToggleInteractWidget (Variables|/Game/EscapeGame/Blueprints/BP_PlayerCharacter.BP_PlayerCharacter_C|GetHUD _asbp_player_character) "Hidden"))

(fn ConstructionScript)

(fn IsComponentInteractive
  (params (Comp :type Actor%20Component%20Object%20Reference))
  (if (!= (Class|Furniture|FindDrawerIndexbyComponent Comp) -1)
    (return true)
    (else
      (return (!= (Class|Furniture|FindCabinetDoorIndexbyComponent Comp) -1)))))

(fn GetInteractionText
  (params (Comp :type Actor%20Component%20Object%20Reference))
  (bind _returnvalue (Class|Furniture|FindCabinetDoorIndexbyComponent Comp))
  (bind _returnvalue_2 (Class|Furniture|FindDrawerIndexbyComponent Comp))
  (if (!= _returnvalue_2 -1)
    (return (Utilities|Select :Index (.State (Utilities|Struct|BreakDrawer (Utilities|Array|Get(acopy) (Variables|Default|GetDrawers) _returnvalue_2))) :Opened "to Close Drawer" :Closed "to Open Drawer"))
    (elif (!= _returnvalue -1)
      (return (Utilities|Select :Index (.State (Utilities|Struct|BreakCabinetDoor (Utilities|Array|Get(acopy) (Variables|Default|GetCabinetDoors) _returnvalue))) :Opened "to Close Cabinet Door" :Closed "to Open Cabinet Door"))
      (else
        (return (Variables|Default|GetInteractionTextErrString))))))
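; Blueprint helper that looks up icon textures for input keys, action mappings and axis mappings.
; GetKeyTexture scans data table rows for a matching key and returns that row's texture with a Found flag.
; The action and axis functions run it over each mapping and return the first hit.
; InputMode selects the table, but both shown options point to the keyboard table.
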(fn GetKeyTexture
  (params (Key :type Key%20Structure :default "None") (InputMode :type Byte))
  (bind _returnvalue (Utilities|Select :Index InputMode :Option%200 "/Game/EscapeGame/Database/Input/InputActionTextures_keyboard_DataTable.InputActionTextures_keyboard_DataTable" :Option%201 "/Game/EscapeGame/Database/Input/InputActionTextures_keyboard_DataTable.InputActionTextures_keyboard_DataTable"))
  (bind _outrownames (DataTable|GetDataTableRowNames _returnvalue))
  (bind _array_element (Utilities|Array|ForEachLoopwithBreak _outrownames :!label _label)
    (:LoopBody
      (bind _returnvalue_2 (Utilities|GetDataTableRow _returnvalue _array_element)
        (:then
          (if (== (.Key (Utilities|Struct|BreakInputActionTexture_Struct _returnvalue_2)) Key)
            (LocalVariables|SetFound _array_element)
            (goto _label Break)))))
    (:Completed
      (if (Utilities|Name|NotEqual(Name) (LocalVariables|GetFound) "None")
        (bind _returnvalue_3 (Utilities|GetDataTableRow _returnvalue (LocalVariables|GetFound))
          (:then
            (return (.Texture (Utilities|Struct|BreakInputActionTexture_Struct _returnvalue_3)) true)))
        (else
          (return 0 false))))))

(fn FindKeyTexturefromInputAction
  (params (InputActions :type Array%20of%20Input%20Action%20Key%20Mapping%20Structures) (InputMode :type Byte))
  (bind _array_index (Utilities|Array|ForEachLoopwithBreak InputActions :!label _label)
    (:LoopBody
      (bind (_texture2d _bfound) (CallFunction|GetKeyTexture (Utilities|Struct|BreakInputActionKeyMapping (Utilities|Array|Get(acopy) InputActions _array_index)) InputMode))
      (if _bfound
        (LocalVariables|SetbFound true)
        (LocalVariables|SetTex2D _texture2d)
        (goto _label Break)))
    (:Completed
      (return (LocalVariables|GetTex2D) (LocalVariables|GetbFound)))))

(fn FindKeyTexturefromInputAxis
  (params (InputAxis :type Array%20of%20Input%20Axis%20Key%20Mapping%20Structures) (InputMode :type Byte))
  (bind _array_index (Utilities|Array|ForEachLoopwithBreak InputAxis :!label _label)
    (:LoopBody
      (bind (_texture2d _bfound) (CallFunction|GetKeyTexture (Utilities|Struct|BreakInputAxisKeyMapping (Utilities|Array|Get(acopy) InputAxis _array_index)) InputMode))
      (if _bfound
        (LocalVariables|SetbFound true)
        (LocalVariables|SetTex2D _texture2d)
        (goto _label Break)))
    (:Completed
      (return (LocalVariables|GetTex2D) (LocalVariables|GetbFound)))))
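; Player character for an escape game that creates the main HUD, toggles crouching and checks for held keys.
; BeginPlay shows the HUD and stores the camera's start location, while the Crouch input switches between built-in Crouch and UnCrouch.
; HasKey searches inventory items for key data with a matching ID.
; A timeline-driven camera lowering for crouch is present but disconnected, so it never runs.
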(event EventBeginPlay
  (bind _returnvalue (UserInterface|CreateWidget "/Game/EscapeGame/UI/WBP_MainHUD.WBP_MainHUD_C"))
  (bind _output_get (Variables|Default|SetHUD _returnvalue))
  (UserInterface|Viewport|AddtoViewport _output_get 0)
  (Variables|Default|SetPlayerCameraStartLocation (Variables|/Script/Engine.SceneComponent|GetRelativeLocation (Variables|Default|GetCameraComp))))

(event Input|ActionEvents|InputActionCrouch
  (params (Key :type Key%20Structure :default "None"))
  (:Pressed
    (if (Variables|Default|GetbIsCrouched)
      (Character|UnCrouch)
      (else
        (Character|Crouch)))))

(event Input|ActionEvents|InputActionInventory
  (params (Key :type Key%20Structure :default "None")))

(fn ConstructionScript)

(fn HasKey
  (params (Key :type Guid%20Structure))
  (bind _array_element (Utilities|Array|ForEachLoopwithBreak (Variables|/Script/EscapeGame.InventoryComponent|GetItems (Variables|Default|GetInventoryComponent)) :!label _label)
    (:LoopBody
      (bind _asbp_key_item_data (Utilities|Casting|CastToBP_Key_ItemData _array_element))
      (if (== (Variables|/Game/EscapeGame/Blueprints/Items/BP_Key_ItemData.BP_Key_ItemData_C|GetKeyID _asbp_key_item_data) Key)
        (LocalVariables|SetKeyFound true)
        (goto _label Break)))
    (:Completed
      (return (LocalVariables|GetKeyFound)))))
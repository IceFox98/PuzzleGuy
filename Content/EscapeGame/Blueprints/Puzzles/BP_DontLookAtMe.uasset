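; Puzzle actor for the escape game whose text hides or shows depending on the direction the player aims.
; BeginPlay caches the controlled pawn of player 0 as a PlayerCharacter.
; Each Tick dots the player's aim forward vector with the TextRender's forward vector, hiding the text above MaxDotAngle.
; The test compares directions only, ignoring position and line of sight.
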(event EventTick
  (params (DeltaSeconds :type Float%20%28single-precision%29))
  (bind _output_get (Variables|Default|SetMustHide (> (Math|Vector|DotProduct (Math|Vector|GetForwardVector (Pawn|GetBaseAimRotation (Variables|Default|GetPlayerRef))) (Math|Vector|GetForwardVector (Transformation|GetWorldRotation (Variables|Default|GetTextRender)))) (Variables|Default|GetMaxDotAngle))))
  (Rendering|SetVisibility (Variables|Default|GetTextRender) (not _output_get) true))

(event EventBeginPlay
  (bind _asplayer_character (Utilities|Casting|CastToPlayerCharacter (Pawn|GetControlledPawn (Game|GetPlayerController 0))))
  (Variables|Default|SetPlayerRef _asplayer_character))

(fn ConstructionScript)
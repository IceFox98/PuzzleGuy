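; BP_GridStart is an interactable button that starts a memory grid puzzle in the escape game.
; On interact, if the referenced grid is valid and not yet completed, it raises the player's interaction range and calls Start on the BP_MemoryGrid.
; Only the Button component is interactive, highlighted through custom depth while focused, with empty interaction text.
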(event EventBeginPlay)

(event Collision|EventActorBeginOverlap
  (params (OtherActor :type Actor%20Object%20Reference)))

(event EventTick
  (params (DeltaSeconds :type Float%20%28single-precision%29)))

(event EventOnInteract
  (params (Controller :type Controller%20Object%20Reference) (Comp :type Actor%20Component%20Object%20Reference))
  (bind _gridref (Variables|Default|GetGridRef))
  (Utilities|IsValid _gridref
    (:Is%20Valid
      (if (not (Variables|/Script/EscapeGame.PuzzleBase|GetbIsCompleted _gridref))
        (bind _asbp_player_character (Utilities|Casting|CastToBP_PlayerCharacter (Pawn|GetControlledPawn Controller)))
        (Class|InteractionComponent|ChangeRange (Variables|/Script/EscapeGame.PlayerCharacter|GetInteractionComponent _asbp_player_character) 5e+03)
        (bind _asbp_memory_grid (Utilities|Casting|CastToBP_MemoryGrid (Variables|Default|GetGridRef)))
        (Class|MemoryGrid|Start _asbp_memory_grid)
        (Development|PrintString "Starting...")))
    (:Is%20Not%20Valid
      (Development|PrintString "GridRef Missing" true true "(R=1.000000,G=0.004341,B=0.000000,A=1.000000)"))))

(event EventOnBeginFocus
  (params (Controller :type Controller%20Object%20Reference) (Comp :type Actor%20Component%20Object%20Reference))
  (Rendering|SetRenderCustomDepth (Variables|Default|GetButton) true))

(event EventOnEndFocus
  (params (Controller :type Controller%20Object%20Reference))
  (Rendering|SetRenderCustomDepth (Variables|Default|GetButton) false))

(fn ConstructionScript)

(fn GetInteractionText
  (params (Comp :type Actor%20Component%20Object%20Reference))
  (return ""))

(fn IsComponentInteractive
  (params (Comp :type Actor%20Component%20Object%20Reference))
  (return (== Comp (Variables|Default|GetButton))))
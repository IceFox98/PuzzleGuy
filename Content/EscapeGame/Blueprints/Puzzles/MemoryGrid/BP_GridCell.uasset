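; Grid cell actor for the MemoryGrid puzzle in EscapeGame, giving color feedback when focused or guessed.
; At BeginPlay it creates and stores a dynamic material instance from its mesh's first material.
; Focus begin and end events call ChangeColor only while the cell is unlocked, whereas OnGuessed recolors it regardless.
; IsComponentInteractive reports the cell as interactive whenever it is not Locked.
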(event Custom|OnGuessed
  (Class|GridCell|ChangeColor "Guessed"))

(event EventBeginPlay
  (bind _returnvalue (Rendering|Material|CreateDynamicMaterialInstance (Variables|Character|GetMesh) 0 (Rendering|Material|GetMaterial (Variables|Character|GetMesh) 0) "None" :!class /Script/Engine.PrimitiveComponent))
  (Variables|Default|SetDynamicMatInstance _returnvalue))

(event Collision|EventActorBeginOverlap
  (params (OtherActor :type Actor%20Object%20Reference)))

(event EventTick
  (params (DeltaSeconds :type Float%20%28single-precision%29)))

(event EventOnBeginFocus
  (params (Controller :type Controller%20Object%20Reference) (Comp :type Actor%20Component%20Object%20Reference))
  (if (not (Variables|Default|GetLocked))
    (Class|GridCell|ChangeColor "BeginFocus")))

(event EventOnEndFocus
  (params (Controller :type Controller%20Object%20Reference))
  (if (not (Variables|Default|GetLocked))
    (Class|GridCell|ChangeColor "EndFocus")))

(fn ConstructionScript)

(fn IsComponentInteractive
  (params (Comp :type Actor%20Component%20Object%20Reference))
  (return (not (Variables|Default|GetLocked))))
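; Memory grid puzzle that flashes a random cell sequence for the player to guess, completing once the sequence is empty.
; A looping timer highlights cells one by one, then after a delay clears and unlocks them all.
; Correct guesses lock and notify their cell, while a wrong guess resets the grid.
; The construction script builds a preview mesh grid, destroyed on BeginPlay.
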(event Custom|ShowCell
  (Default|ChangeColor (Utilities|Array|Get(acopy) (Variables|Default|GetCells) (Utilities|Array|Get(acopy) (Variables|Default|GetRandomSequence) (Variables|Default|GetShowSequenceIndex))) "BeginFocus")
  (Math|Integer|IncrementInt (Variables|Default|GetShowSequenceIndex)
    (:%20%20
      (if (>= (Variables|Default|GetShowSequenceIndex) (Utilities|Array|Length (Variables|Default|GetRandomSequence)))
        (Utilities|Time|ClearandInvalidateTimerbyHandle (Variables|Default|GetSequenceTimer))
        ;[1 1 1] Hide Sequence and unlock cell interactions
        (Utilities|FlowControl|Delay 2.0)
        (for _array_element (Variables|Default|GetCells)
          (Variables|/Script/EscapeGame.GridCell|SetLocked _array_element false)
          (Default|ChangeColor _array_element "EndFocus"))))))

(event EventBeginPlay
  (for _array_element (Variables|Default|GetPreviewMeshes)
    (Components|DestroyComponent _array_element)))

(event EventOnWrongSequence
  (Development|PrintString "Wrong sequence!")
  (Class|MemoryGrid|ResetCells true)
  (Variables|Default|SetShowSequenceIndex 0)
  (CallFunction|GetPlayerCharacter))

(event EventShowSequence
  (bind _returnvalue (Utilities|Time|SetTimerbyEvent (delegate Custom|ShowCell) (Variables|Default|GetGenerationCellsDelay) true))
  (Variables|Default|SetSequenceTimer _returnvalue))

(event EventOnCellGuessed
  (params (GuessedCell :type Grid%20Cell%20Object%20Reference))
  (Variables|/Script/EscapeGame.GridCell|SetLocked GuessedCell true)
  (bind _asbp_grid_cell (Utilities|Casting|CastToBP_GridCell GuessedCell))
  (Default|OnGuessed _asbp_grid_cell)
  (if (Utilities|Array|IsEmpty (Variables|Default|GetRandomSequence))
    (Development|PrintString "Victory!")
    (Class|PuzzleBase|OnCompleted)))

(fn ConstructionScript
  (for _index (range 0 (- (Variables|Default|GetGridRows) 1))
    (for _index_2 (range 0 (- (Variables|Default|GetGridColumns) 1))
      (bind _returnvalue (AddComponent|AddStaticMeshComponent false (Math|Transform|MakeTransform (Math|Vector|MakeVector (* (Variables|Default|GetCellSpacing) _index) (* _index_2 (Variables|Default|GetCellSpacing)) 0.0) "0, 0, 0" "3.000000,3.000000,0.300000")))
      (Utilities|Array|AddUnique (Variables|Default|GetPreviewMeshes) _returnvalue))))
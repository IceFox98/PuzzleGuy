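; BP_GridStart is the interactable that starts the Memory Grid puzzle in the escape game.
; On interact, the parent OnInteract sets PuzzleIsReady, which gates the rest of the logic.
; When ready, it changes the player's InteractionComponent range to a much larger value, then casts PuzzleRef to BP_MemoryGrid, calls Start and prints a status message.
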(event EventBeginPlay
  (|CallParentFunction) ; This node is disabled and will not be called.\nDrag off pins to build functionality.
)

(event Collision|EventActorBeginOverlap
  (params (OtherActor :type Actor%20Object%20Reference))
  (|CallParentFunction OtherActor) ; This node is disabled and will not be called.\nDrag off pins to build functionality.
)

(event EventTick
  (params (DeltaSeconds :type Float%20%28single-precision%29))
  (|CallParentFunction DeltaSeconds) ; This node is disabled and will not be called.\nDrag off pins to build functionality.
)

(event EventOnInteract
  (params (Controller :type Controller%20Object%20Reference) (Comp :type Actor%20Component%20Object%20Reference))
  (|CallParentFunction Controller Comp)
  (if (Variables|Default|GetbPuzzleIsReady)
    (bind _asbp_player_character (Utilities|Casting|CastToBP_PlayerCharacter (Pawn|GetControlledPawn Controller)))
    (Class|InteractionComponent|ChangeRange (Variables|/Script/EscapeGame.PlayerCharacter|GetInteractionComponent _asbp_player_character) 5e+03)
    (bind _asbp_memory_grid (Utilities|Casting|CastToBP_MemoryGrid (Variables|Default|GetPuzzleRef)))
    (Class|MemoryGrid|Start _asbp_memory_grid)
    (Development|PrintString "Starting...")))

(fn ConstructionScript
  (|CallParentFunction))
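; BP_PuzzleStart is an interactive button actor for a linked puzzle in the escape game.
; On interaction it sets PuzzleIsReady to true only if the referenced puzzle is not completed, or prints an error when the reference is missing.
; Only the Button component is interactive, and it highlights through custom depth while focused, with empty interaction text.
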(event EventBeginPlay)

(event Collision|EventActorBeginOverlap
  (params (OtherActor :type Actor%20Object%20Reference)))

(event EventTick
  (params (DeltaSeconds :type Float%20%28single-precision%29)))

(event EventOnInteract
  (params (Controller :type Controller%20Object%20Reference) (Comp :type Actor%20Component%20Object%20Reference))
  (bind _puzzleref (Variables|Default|GetPuzzleRef))
  (Utilities|IsValid _puzzleref
    (:Is%20Valid
      (Variables|Default|SetbPuzzleIsReady (not (Variables|/Script/EscapeGame.PuzzleBase|GetbIsCompleted _puzzleref))))
    (:Is%20Not%20Valid
      (Development|PrintString "GridRef Missing" true true "(R=1.000000,G=0.004341,B=0.000000,A=1.000000)"))))

(event EventOnBeginFocus
  (params (Controller :type Controller%20Object%20Reference) (Comp :type Actor%20Component%20Object%20Reference))
  (Rendering|SetRenderCustomDepth (Variables|Default|GetButton) true))

(event EventOnEndFocus
  (params (Controller :type Controller%20Object%20Reference))
  (Rendering|SetRenderCustomDepth (Variables|Default|GetButton) false))

(fn ConstructionScript)

(fn GetInteractionText
  (params (Comp :type Actor%20Component%20Object%20Reference))
  (return ""))

(fn IsComponentInteractive
  (params (Comp :type Actor%20Component%20Object%20Reference))
  (return (== Comp (Variables|Default|GetButton))))
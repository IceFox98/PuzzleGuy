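; BP_ExitButton is a maze puzzle button that sinks when physically hit and triggers a linked actor.
; A component hit on the button fires once, guarded by a Pressed flag, and plays a timeline that lerps the button down from its starting relative position.
; It then calls OnInteract on ActorToTrigger through a cast to Interactable.
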(event OnComponentHit(Button)
  (params (HitComponent :type Primitive%20Component%20Object%20Reference) (OtherActor :type Actor%20Object%20Reference) (OtherComp :type Primitive%20Component%20Object%20Reference) (NormalImpulse :type Vector :default "0, 0, 0") (Hit :type Hit%20Result%20Structure%20%28by%20ref%29))
  (if (not (Variables|Default|GetbPressed))
    (Utilities|FlowControl|Sequence
      (:then_0
        (bind _alpha (Timeline|PressButton Play)
          (:Update
            (Transformation|SetRelativeLocation (Variables|Default|GetButton) (Math|Vector|Lerp(Vector) (Variables|Default|GetInitialLocation) (Variables|Default|GetEndLocation) _alpha) false false))))
      (:then_1
        (Variables|Default|SetbPressed true)
        (bind _asinteractable (Utilities|Casting|CastToInteractable (Variables|Default|GetActorToTrigger)))
        (Class|Interactable|OnInteract _asinteractable)))))

(event EventBeginPlay
  (bind _output_get (Variables|Default|SetInitialLocation (Variables|/Script/Engine.SceneComponent|GetRelativeLocation (Variables|Default|GetButton))))
  (Variables|Default|SetEndLocation (- _output_get "0,0,30.000000")))

(fn ConstructionScript)
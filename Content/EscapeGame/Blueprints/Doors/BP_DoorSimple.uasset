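; Simple interactive door for the escape game that swings open or closed when the player interacts with it.
; Interacting flips the Opened/Closed state and plays or reverses the OpenCloseDoor timeline, which scales its curve by MaxOpenAngle to set the door mesh's relative yaw.
; Focus events show or hide the player HUD's interact prompt, with text chosen by the current state.
; Only the SMDoor component reports as interactive.
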(event EventOnBeginFocus
  (params (Controller :type Controller%20Object%20Reference) (Comp :type Actor%20Component%20Object%20Reference))
  (bind _returnvalue (CallFunction|GetInteractionText Comp))
  (if (Utilities|Enum|NotEqual(Enum) _returnvalue (Variables|Default|GetInteractionTextErrString))
    (bind _asbp_player_character (Utilities|Casting|CastToBP_PlayerCharacter (Pawn|GetControlledPawn Controller)))
    (Default|ToggleInteractWidget (Variables|/Game/EscapeGame/Blueprints/BP_PlayerCharacter.BP_PlayerCharacter_C|GetHUD _asbp_player_character) "Visible")
    (Default|SetInteractText (Variables|/Game/EscapeGame/Blueprints/BP_PlayerCharacter.BP_PlayerCharacter_C|GetHUD _asbp_player_character) _returnvalue)))

(event EventOnInteract
  (params (Controller :type Controller%20Object%20Reference) (Comp :type Actor%20Component%20Object%20Reference))
  (bind _sm_door (Variables|Default|GetSM_Door))
  (bind _relativerotation (Variables|/Script/Engine.SceneComponent|GetRelativeRotation _sm_door))
  (switch Utilities|FlowControl|Switch|SwitchonOpenClosed_Enum (Variables|Default|GetState)
    (:NewEnumerator0
      (Variables|Default|SetState (Utilities|Select :Index (Variables|Default|GetState) :NewEnumerator0 "NewEnumerator1" :NewEnumerator1 "NewEnumerator0"))
      (bind _openangle (Timeline|OpenCloseDoor Reverse)
        (:Update
          (Transformation|SetRelativeRotation (Variables|Default|GetSM_Door) (Math|Rotator|MakeRotator (.roll _relativerotation) (.pitch _relativerotation) (* _openangle (Variables|Default|GetMaxOpenAngle))) false false))))
    (:NewEnumerator1
      (Variables|Default|SetState (Utilities|Select :Index (Variables|Default|GetState) :NewEnumerator0 "NewEnumerator1" :NewEnumerator1 "NewEnumerator0"))
      (Timeline|OpenCloseDoor Play))))

(event EventOnEndFocus
  (params (Controller :type Controller%20Object%20Reference))
  (bind _asbp_player_character (Utilities|Casting|CastToBP_PlayerCharacter (Pawn|GetControlledPawn Controller)))
  (Default|ToggleInteractWidget (Variables|/Game/EscapeGame/Blueprints/BP_PlayerCharacter.BP_PlayerCharacter_C|GetHUD _asbp_player_character) "Hidden"))

(fn ConstructionScript)

(fn GetInteractionText
  (params (Comp :type Actor%20Component%20Object%20Reference))
  (return (Utilities|Select :Index (Variables|Default|GetState) :NewEnumerator0 "to Close the Door" :NewEnumerator1 "to Open the Door")))

(fn IsComponentInteractive
  (params (Comp :type Actor%20Component%20Object%20Reference))
  (return (== Comp (Variables|Default|GetSM_Door))))
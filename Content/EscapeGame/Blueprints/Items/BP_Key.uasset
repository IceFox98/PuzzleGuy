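; BP_Key is an interactable key pickup that adds a key item to an inventory.
; On interaction it adds its ItemClass through GetInventory, casts the new item to BP_Key_ItemData and copies its KeyID onto it.
; A sequence then runs the parent OnInteract logic, even if that cast fails.
; The interaction prompt is hardcoded to describe a drawer key.
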(event EventBeginPlay
  (|CallParentFunction) ; This node is disabled and will not be called.\nDrag off pins to build functionality.
)

(event Collision|EventActorBeginOverlap
  (params (OtherActor :type Actor%20Object%20Reference))
  (|CallParentFunction OtherActor) ; This node is disabled and will not be called.\nDrag off pins to build functionality.
)

(event EventTick
  (params (DeltaSeconds :type Float%20%28single-precision%29))
  (|CallParentFunction DeltaSeconds) ; This node is disabled and will not be called.\nDrag off pins to build functionality.
)

(event EventOnInteract
  (params (Controller :type Controller%20Object%20Reference) (Comp :type Actor%20Component%20Object%20Reference))
  (Utilities|FlowControl|Sequence
    (:then_0
      (bind _inventory_component (CallFunction|GetInventory))
      (bind _returnvalue (Class|InventoryComponent|AddItem _inventory_component (Variables|Default|GetItemClass)))
      (bind _asbp_key_item_data (Utilities|Casting|CastToBP_Key_ItemData _returnvalue))
      (Variables|/Game/EscapeGame/Blueprints/Items/BP_Key_ItemData.BP_Key_ItemData_C|SetKeyID _asbp_key_item_data (Variables|Key|GetKeyID)))
    (:then_1
      (|CallParentFunction Controller Comp))))

(fn ConstructionScript
  (|CallParentFunction))

(fn GetInteractionText
  (params (Comp :type Actor%20Component%20Object%20Reference))
  (return "to Pickup Drawer Key"))
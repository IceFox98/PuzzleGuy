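; BP_Inventory_Item is an interactable item actor in the escape game that is destroyed when interacted with; no inventory transfer happens here.
; On focus, it casts the controller's pawn to BP_PlayerCharacter, shows the HUD interact widget and sets its text from GetInteractionText.
; Losing focus hides the widget.
; Every component reports as interactive, and the interaction text returned here is empty.
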(event EventBeginPlay)

(event EventOnBeginFocus
  (params (Controller :type Controller%20Object%20Reference) (Comp :type Actor%20Component%20Object%20Reference))
  (bind _returnvalue (CallFunction|GetInteractionText Comp))
  (bind _asbp_player_character (Utilities|Casting|CastToBP_PlayerCharacter (Pawn|GetControlledPawn Controller)))
  (Default|ToggleInteractWidget (Variables|/Game/EscapeGame/Blueprints/BP_PlayerCharacter.BP_PlayerCharacter_C|GetHUD _asbp_player_character) "Visible")
  (Default|SetInteractText (Variables|/Game/EscapeGame/Blueprints/BP_PlayerCharacter.BP_PlayerCharacter_C|GetHUD _asbp_player_character) _returnvalue))

(event EventTick
  (params (DeltaSeconds :type Float%20%28single-precision%29)))

(event Collision|EventActorBeginOverlap
  (params (OtherActor :type Actor%20Object%20Reference)))

(event EventOnEndFocus
  (params (Controller :type Controller%20Object%20Reference))
  (bind _asbp_player_character (Utilities|Casting|CastToBP_PlayerCharacter (Pawn|GetControlledPawn Controller)))
  (Default|ToggleInteractWidget (Variables|/Game/EscapeGame/Blueprints/BP_PlayerCharacter.BP_PlayerCharacter_C|GetHUD _asbp_player_character) "Hidden"))

(event EventOnInteract
  (params (Controller :type Controller%20Object%20Reference) (Comp :type Actor%20Component%20Object%20Reference))
  (Actor|DestroyActor))

(fn ConstructionScript)

(fn GetInteractionText
  (params (Comp :type Actor%20Component%20Object%20Reference))
  (return ""))

(fn IsComponentInteractive
  (params (Comp :type Actor%20Component%20Object%20Reference))
  (return true))